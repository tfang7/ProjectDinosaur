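; IdleGameController is the controller for an idle clicker game, tracking money and clicks.
; On BeginPlay it resets the click count and adds a HUD widget to the viewport.
; A left click adds click income to Money, while Tick accumulates time and adds idle income every two seconds.
; The construction script sets default incomes, multipliers and couch level, though the multipliers and couch level are not yet used.
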(event `self.ReceiveBeginPlay`
  (set `self.Clicks` 0)
  (bind _returnvalue (`|CreateWidget` "/Game/UI/HUD.HUD_C"))
  (bind _output_get (set `self.HUDReference` _returnvalue))
  (`UserWidget.AddToViewport` _output_get 0))

(event `self.ReceiveTick`
  (params (DeltaSeconds :type "Float (single-precision)"))
  (bind _output_get (set `self.DeltaTime` (+ DeltaSeconds (`self.DeltaTime`))))
  (if (>= _output_get 2.0)
    (set `self.Money` (+ (`self.Money`) (`self.IdleIncome`)))
    (set `self.DeltaTime` 0.0)))

(event `Key|LeftMouseButton`
  (params (Key :type "Key Structure"))
  (:`Pressed`
    (set `self.Clicks` (+ (`self.Clicks`) 1))
    (set `self.Money` (+ (`self.Money`) (`self.ClickIncome`)))))

(fn `UserConstructionScript`
  ;[1 1 1] Read values from save file later
  (set `self.ClickIncome` 10.0)
  (set `self.IdleIncome` 0.0)
  (set `self.IdleMultiplier` 1.0)
  (set `self.ClickMultiplier` 1.0)
  (set `self.CouchLevel` 0))